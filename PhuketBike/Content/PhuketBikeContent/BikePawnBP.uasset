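; Bike pawn for a dodging game: when flagged as the player, it moves along Y with Up/Down and loses a life on overlapping an NPC bike.
; Tick chains smoothed steering, Y clamping, stopping on death and speed ramp-up, easing MovementSpeed toward its target without applying it here.
; The ramp's speed-cap check is disconnected, so target speed rises unbounded while alive.
; Enter resets lives and speed after death; Escape exits.
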(event `Key|Escape`
  (params (Key :type "Key Structure"))
  (:`Released`
    (`KismetSystemLibrary.ExecuteConsoleCommand` "exit" null)))

(event `Key|Enter`
  (params (Key :type "Key Structure"))
  (:`Pressed`
    (if (<= (`self.Life`) 0)
      (`self.ResetGame`))))

(event `Key|Up`
  (params (Key :type "Key Structure"))
  (:`Pressed`
    (set `self.inputGoingUp` true))
  (:`Released`
    (set `self.inputGoingUp` false)))

(event `Key|Down`
  (params (Key :type "Key Structure"))
  (:`Pressed`
    (set `self.inputGoingDown` true))
  (:`Released`
    (set `self.inputGoingDown` false)))

(event `self.ReceiveActorBeginOverlap`
  (params (OtherActor :type "Actor Object Reference"))
  (if (`self.isPlayer`)
    (cast `/Game/PhuketBikeContent/BikePawnBP_NPC` OtherActor)
    (set `self.Life` (- (`self.Life`) 1))
    (`KismetSystemLibrary.PrintString` (`KismetStringLibrary.Conv_IntToString` (`self.Life`)))))

(event `self.ReceiveTick`
  (params (DeltaSeconds :type "Float (single-precision)"))
  (if (`self.isPlayer`)
    (`self.MovePlayerByInput` DeltaSeconds
      (:`OutExec`
        (`self.LimitPlayerLocation`
          (:`ExecOut`
            (`self.StopPlayerMovementAfterDeath`
              (:`ExecOut`
                (`self.GradualIncreasingPlayerSpeedAsTimeGoesOn` DeltaSeconds
                  (:`ExecOut`
                    (`self.SpeedAdjustment` DeltaSeconds)))))))))))

(fn `ResetGame`
  (set `self.Life` 3)
  (set `self.movementSpeed` 0.0)
  (set `self.targetMovementSpeed` 100.0))

(fn `UserConstructionScript`)